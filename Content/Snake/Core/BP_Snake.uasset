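; BP_Snake is the snake game Blueprint that handles the HUD and game-over screen.
; BeginPlay shows the W_MainGame widget, and UpdateScore passes apple count and time to its score sub-widget.
; GameOver shows the cursor and swaps the HUD for W_GameOver, filled with the final time and apples eaten.
; Snake and apple spawn calls sit in a disconnected chain that never runs.
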(event EventGameOver
  (Variables|/Script/Engine.PlayerController|SetbShowMouseCursor (Game|GetPlayerController 0) true)
  (Widget|RemovefromParent (Variables|Default|GetMainWidget))
  (bind _returnvalue (UserInterface|CreateWidget "/Game/Snake/Widgets/W_GameOver.W_GameOver_C"))
  (Variables|Default|SetGameOverWidget _returnvalue)
  (UserInterface|Viewport|AddtoViewport (Variables|Default|GetGameOverWidget) 0)
  (Default|SetGameScore (Variables|/Game/Snake/Widgets/W_GameOver.W_GameOver_C|GetW_GameScore (Variables|Default|GetGameOverWidget)) (Variables|Default|GetGameTimer) (Variables|Default|GetEatenApples)))

(event EventUpdateScore
  (params (apple :type Integer) (timer :type Float%20%28single-precision%29))
  (Default|SetGameScore (Variables|/Game/Snake/Widgets/W_MainGame.W_MainGame_C|GetW_GameScore (Variables|Default|GetMainWidget)) timer apple))

(event EventBeginPlay
  (bind _returnvalue (UserInterface|CreateWidget "/Game/Snake/Widgets/W_MainGame.W_MainGame_C"))
  (Variables|Default|SetMainWidget _returnvalue)
  (UserInterface|Viewport|AddtoViewport (Variables|Default|GetMainWidget) 0))

(fn ConstructionScript)